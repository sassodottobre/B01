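; BP_TorreAlien is an alien tower that the rover activates by entering its Activationzone.
; On overlap, an unactivated tower waits two seconds, without rechecking that the rover remains, then sets IsActivated and prints it.
; It then calls TorreAttivata on GM_RoverGameMode, hides the green light beam mesh and shows the red inside light.
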(event `self.ReceiveTick`
  (params (DeltaSeconds :type "Float (single-precision)")))

(event `self.activationzone.OnComponentBeginOverlap`
  (params (OverlappedComponent :type "PrimitiveComponent Object Reference") (OtherActor :type "Actor Object Reference") (OtherComp :type "PrimitiveComponent Object Reference") (OtherBodyIndex :type Integer) (bFromSweep :type Boolean) (SweepResult :type "HitResult Structure (by ref)"))
  (if (!= (`self.IsActivated`) true)
    (cast `/Game/BluePrint/BP_Rover` OtherActor)
    (`KismetSystemLibrary.Delay` 2.0)
    (if (not false)
      (bind _output_get (set `self.IsActivated` true))
      (`KismetSystemLibrary.PrintString` (`KismetStringLibrary.Conv_BoolToString` _output_get))
      ;[1 1 1] Cast To torriattivata
      (bind _asgm_rover_game_mode (cast `/Game/BluePrint/GM_RoverGameMode` (`GameplayStatics.GetGameMode`)))
      (`/Game/BluePrint/GM_RoverGameMode.TorreAttivata` _asgm_rover_game_mode)
      ;[1 1 1] despawn green light
      (`SceneComponent.SetVisibility` (`self.LIghtBeamMesh`) false false)
      ;[1 1 1] spawn red light
      (`SceneComponent.SetVisibility` (`self.insidelight`) true false))))

(fn `UserConstructionScript`)