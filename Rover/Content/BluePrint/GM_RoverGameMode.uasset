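; Game mode for the rover game that tracks tower activations and triggers the win condition.
; TorreAttivata increments the TorriAttivate counter and calls GameOverWin when it reaches four.
; GameOverWin adds the WBP_GameWin widget to the viewport, switches the player controller to UI-only input and pauses the game.
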(fn `GameOverWin`
  (bind _returnvalue (`|CreateWidget` "/Game/BluePrint/WBP_GameWin.WBP_GameWin_C"))
  (`UserWidget.AddToViewport` _returnvalue 0)
  (bind _returnvalue_2 (`InputDeviceLibrary.GetPlayerControllerFromInputDevice` (struct)))
  (`WidgetBlueprintLibrary.SetInputMode_UIOnlyEx` _returnvalue_2 null)
  (`GameplayStatics.SetGamePaused` true))

(fn `TorreAttivata`
  (bind _output_get (set `self.TorriAttivate` (+ (`self.TorriAttivate`) 1)))
  (if (== _output_get 4)
    (`self.GameOverWin`)))

(fn `UserConstructionScript`)